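; BP_TestActor is a test actor that changes the color of its static mesh when overlapped by components tagged "ChangeColor".
; Begin overlap applies the InLinearColor value, and end overlap sets a fixed cyan.
; Both events call SetColor, which converts the color to a vector and writes it to the "Color" parameter on the mesh's materials.
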(event OnComponentBeginOverlap(StaticMesh)
  (params (OverlappedComponent :type Primitive%20Component%20Object%20Reference) (OtherActor :type Actor%20Object%20Reference) (OtherComp :type Primitive%20Component%20Object%20Reference) (OtherBodyIndex :type Integer) (bFromSweep :type Boolean) (SweepResult :type Hit%20Result%20Structure%20%28by%20ref%29))
  (if (Components|ComponentHasTag OtherComp "ChangeColor")
    (CallFunction|SetColor (Variables|Default|GetIn%20Linear%20Color))))

(event OnComponentEndOverlap(StaticMesh)
  (params (OverlappedComponent :type Primitive%20Component%20Object%20Reference) (OtherActor :type Actor%20Object%20Reference) (OtherComp :type Primitive%20Component%20Object%20Reference) (OtherBodyIndex :type Integer))
  (if (Components|ComponentHasTag OtherComp "ChangeColor")
    (CallFunction|SetColor "(R=0.104167,G=0.944886,B=1.000000,A=1.000000)")))

(fn ConstructionScript)

(fn SetColor
  (params (InLinearColor :type Linear%20Color%20Structure))
  (Rendering|Material|SetVectorParameterValueonMaterials (Variables|Default|GetStaticMesh) "Color" (Math|Conversions|ToVector(LinearColor) InLinearColor)))