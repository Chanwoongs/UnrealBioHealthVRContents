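; BP_Label is a text label actor that keeps its TextRender turned toward the player camera every tick.
; AttachToComponent attaches it to a given component with world transform kept, then uses the sign of the root's relative Y to offset the text toward the opposite side and set left or right alignment.
; SetLabelText sets the displayed text.
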(event Custom|LookPlayerCamera
  (Transformation|SetWorldRotation (Variables|Default|GetTextRender) (Math|Rotator|FindLookatRotation (Transformation|GetWorldLocation (Variables|Default|GetTextRender)) (Camera|GetCameraLocation (Game|GetPlayerCameraManager 0))) false false))

(event Custom|AttachToComponent
  (params (AttachTo :type Scene%20Component%20Object%20Reference))
  (bind _textrender (Variables|Default|GetTextRender))
  (bind _textrender_2 (Variables|Default|GetTextRender))
  (Transformation|AttachComponentToComponent AttachTo "None" "KeepWorld" "KeepWorld" "KeepWorld" true)
  (if (> (.y (Variables|/Script/Engine.SceneComponent|GetRelativeLocation (Variables|Default|GetDefaultSceneRoot))) 0.0)
    (Transformation|SetRelativeLocation _textrender "0,-100.000000,40.000000" false false)
    (Rendering|Components|TextRender|SetHorizontalAlignment _textrender_2 "EHTA_Right")
    (else
      (Transformation|SetRelativeLocation _textrender "0,100.000000,40.000000" false false)
      (Rendering|Components|TextRender|SetHorizontalAlignment _textrender_2 "EHTA_Left"))))

(event Custom|SetLabelText
  (params (Value :type Text%20%28by%20ref%29))
  (Rendering|Components|TextRender|SetText (Variables|Default|GetTextRender) Value))

(event EventTick
  (params (DeltaSeconds :type Float%20%28single-precision%29))
  (CallFunction|LookPlayerCamera))

(fn ConstructionScript)