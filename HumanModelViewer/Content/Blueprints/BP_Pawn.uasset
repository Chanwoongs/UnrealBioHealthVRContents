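; BP_Pawn is a preview pawn for a modular human character made of Head, Upper and Lower meshes.
; Mouse input orbits the view and zooms the spring arm within limits, and an event can set the control rotation directly.
; SetGenderData swaps the three meshes from a DT_Human row.
; ZoomInPart isolates one part by enlarging and offsetting it while hiding the others, and ResetZoom restores them.
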(event Custom|SetCameraRotation
  (params (NewParam :type Rotator))
  (Pawn|SetControlRotation (Game|GetPlayerController 0) NewParam))

(event Custom|SetGenderData
  (params (Gender :type Name))
  (bind _returnvalue (Utilities|GetDataTableRow "/Game/Blueprints/DT_Human.DT_Human" Gender)
    (:then
      (Components|StaticMesh|SetStaticMesh (Variables|Default|GetHead) (.Head (Utilities|Struct|BreakS_BodyParts _returnvalue)))
      (Components|StaticMesh|SetStaticMesh (Variables|Default|GetUpper) (.Upper (Utilities|Struct|BreakS_BodyParts _returnvalue)))
      (Components|StaticMesh|SetStaticMesh (Variables|Default|GetLower) (.Lower (Utilities|Struct|BreakS_BodyParts _returnvalue))))))

(event Custom|ZoomInPart
  (params (PartName :type String))
  (Development|SetHiddeninGame (Variables|Default|GetHead) false false)
  (switch string PartName
    (:Head
      (Transformation|SetRelativeTransform (Variables|Default|GetHead) (Math|Transform|MakeTransform "0, 0,-370.000000" "0, 0, 0" "3.000000,3.000000,3.000000") false false)
      (Development|SetHiddeninGame (Variables|Default|GetUpper) true false))
    (:Upper
      (Transformation|SetRelativeTransform (Variables|Default|GetUpper) (Math|Transform|MakeTransform "0, 0,-260.000000" "0, 0, 0" "3.000000,3.000000,3.000000") false false)
      (Development|SetHiddeninGame (Variables|Default|GetHead) true false))
    (:Lower
      (Transformation|SetRelativeTransform (Variables|Default|GetLower) (Math|Transform|MakeTransform "0, 0,-110.000000" "0, 0, 0" "3.000000,3.000000,3.000000") false false)
      (Development|SetHiddeninGame (Variables|Default|GetUpper) true false))))

(event Custom|ResetZoom
  (Transformation|SetRelativeTransform (Variables|Default|GetLower) (Math|Transform|MakeTransform "0, 0, 0") false false)
  (Development|SetHiddeninGame (Variables|Default|GetLower) false false))

(event Input|MouseEvents|MouseX
  (params (AxisValue :type Float%20%28single-precision%29))
  (Pawn|Input|AddControllerYawInput AxisValue))

(event Input|MouseEvents|MouseY
  (params (AxisValue :type Float%20%28single-precision%29))
  (Pawn|Input|AddControllerPitchInput AxisValue))

(event Input|MouseEvents|MouseWheelAxis
  (params (AxisValue :type Float%20%28single-precision%29))
  (bind _springarm (Variables|Default|GetSpringArm))
  (Variables|/Script/Engine.SpringArmComponent|SetTargetArmLength _springarm (Math|Float|Clamp(Float) (+ (* AxisValue -5.0) (Variables|/Script/Engine.SpringArmComponent|GetTargetArmLength _springarm)) 5e+01 4e+02)))

(fn ConstructionScript)